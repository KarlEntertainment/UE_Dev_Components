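; BP_Pick is a pickup item actor that goes into the backpack when interacted with.
; The construction script applies the NewMesh variable to the Cube mesh component, so each instance can set its own appearance.
; InteractEvent adds ItemInfo to the backpack, creates a subtitle saying the named item was added, then destroys the actor.
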(event `self.InteractEvent`
  (`/Game/UnrealFrame/BP_FunctionLibrary.向背包添加内容` (`self.ItemInfo`))
  (`/Game/UnrealFrame/BP_FunctionLibrary.创建字幕` (`|FormatText` "{Name}已添加到背包" (`.物品名字_2_E90D722D4135FAE522DCE3B308F080E3` (break `/Game/UnrealFrame/ST_ItemInfo` (`self.ItemInfo`)))))
  (`self.K2_DestroyActor`))

(fn `UserConstructionScript`
  (`StaticMeshComponent.SetStaticMesh` (`self.Cube`) (`self.New Mesh`)))
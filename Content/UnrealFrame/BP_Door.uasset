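; An interactable hinged door that the player opens and closes with the F key while inside its trigger box.
; Box overlap shows or hides a widget component prompt and enables or disables player input on the actor.
; F flip-flops between playing and reversing a timeline that lerps the door's yaw, while swapping the WBP_InteractWidget prompt text between open and close labels.
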(event `self.Box.OnComponentBeginOverlap`
  (params (OverlappedComponent :type "PrimitiveComponent Object Reference") (OtherActor :type "Actor Object Reference") (OtherComp :type "PrimitiveComponent Object Reference") (OtherBodyIndex :type Integer) (bFromSweep :type Boolean) (SweepResult :type "HitResult Structure (by ref)"))
  (`SceneComponent.SetHiddenInGame` (`self.Widget`) false false)
  (`self.EnableInput` (`GameplayStatics.GetPlayerController` 0)))

(event `self.Box.OnComponentEndOverlap`
  (params (OverlappedComponent :type "PrimitiveComponent Object Reference") (OtherActor :type "Actor Object Reference") (OtherComp :type "PrimitiveComponent Object Reference") (OtherBodyIndex :type Integer))
  (`SceneComponent.SetHiddenInGame` (`self.Widget`) true false)
  (`self.DisableInput` (`GameplayStatics.GetPlayerController` 0)))

(event `Key|F`
  (params (Key :type "Key Structure"))
  (:`Pressed`
    (`/Engine/EditorBlueprintResources/StandardMacros.FlipFlop`
      (:`A`
        (`self.OpenDoor`))
      (:`B`
        (`self.CloseDoor`)))))

(event `OpenDoor`
  (`self.修改文字` "关门")
  (bind (_direction `_新建轨道_0`) (`Timeline|TL_Door` :!label _label)
    (:`Update`
      (`SceneComponent.K2_SetRelativeRotation` (`self.Door`) (`KismetMathLibrary.MakeRotator` 0.0 0.0 (`KismetMathLibrary.Lerp` 0.0 90.0 `_新建轨道_0`)) false false))))

(event `CloseDoor`
  (`self.修改文字` "开门")
  (goto _label :!via `Reverse`))

(event `self.ReceiveBeginPlay`
  (bind _returnvalue (`|CreateWidget` "/Game/UnrealFrame/WBP_InteractWidget.WBP_InteractWidget_C" null "开门"))
  (`WidgetComponent.SetWidget` (`self.Widget`) _returnvalue))

(fn `UserConstructionScript`)

(fn `修改文字`
  (params (InText :type Text))
  (bind _aswbp_interact_widget (cast `/Game/UnrealFrame/WBP_InteractWidget` (`WidgetComponent.GetWidget` (`self.Widget`))))
  (`TextBlock.SetText` (`/Game/UnrealFrame/WBP_InteractWidget.TextBlock_Main` _aswbp_interact_widget) InText))
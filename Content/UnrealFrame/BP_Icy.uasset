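; BP_Icy is an interactable actor whose cube gradually changes its ice effect through a material scalar, 冰冻数值 (freeze value).
; BeginPlay sets the scalar to its minimum, and each InteractEvent raises it a fixed step.
; 修改文字 switches the text to 结冰 (freeze) when a cycle starts and 解冻 (thaw) at the upper limit.
; The limit resets only the stored value, so the material drops back on the next interaction.
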(event `self.ReceiveBeginPlay`
  (`parent.ReceiveBeginPlay`)
  (`MeshComponent.SetScalarParameterValueOnMaterials` (`self.Cube`) "冰冻数值" -70.0))

(event `self.InteractEvent`
  (bind _parameter_value (`self.Parameter Value`))
  (if (<= _parameter_value -70.0)
    (`self.修改文字` "结冰"))
  (bind _output_get (set `self.Parameter Value` (+ _parameter_value 10.0)))
  (`MeshComponent.SetScalarParameterValueOnMaterials` (`self.Cube`) "冰冻数值" _output_get)
  (if (>= _output_get 50.0)
    (`self.修改文字` "解冻")
    (set `self.Parameter Value` -70.0)))

(fn `UserConstructionScript`
  (`parent.UserConstructionScript`))
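; Health component that tracks an actor's current and max health, applying damage and healing, and optionally creates a W_HealthBar widget on BeginPlay.
; Damage subtracts health, flags over-max results as cheating, then checks for death, messaging the owner once.
; Optional low-health and heal events also message the owner, throttled by timer-driven cooldown flags.
; Healing clamps at max health, and a debug flag prints cooldown status.
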(event `self.ReceiveBeginPlay`
  (`self.IfAutoCreateUI`)
  ;[1 1 1] 初始化
  (set `self.CurrentHealth` (`self.MaxHealth`)))

(fn `BasicCureCalculate`
  (params (HealthValue :type "Float (double-precision)"))
  (bind _output_get (set `self.CurrentHealth` (+ (`self.CurrentHealth`) HealthValue)))
  (if (>= _output_get (`self.MaxHealth`))
    (set `self.CurrentHealth` (`self.MaxHealth`))))

(fn `BasicDamageCaculate`
  (params (DamageValue :type "Float (double-precision)"))
  (bind _output_get (set `self.CurrentHealth` (- (`self.CurrentHealth`) DamageValue)))
  (if (>= _output_get (`self.MaxHealth`))
    ;[1 1 1] 如果掉血后血量值大于最大生命值(反作弊)，则恢复到最大生命值
    (set `self.CurrentHealth` (`self.MaxHealth`))
    (`KismetSystemLibrary.PrintString` "检测到作弊者！！！当前对局已结束" true true (struct :`R` 1.0 :`G` 0.016463 :`A` 1.0) 20.0)
    (elif (`self.bUseLowHealthEvent`)
      (if (<= (/ (`self.CurrentHealth`) (`self.MaxHealth`)) (`self.LowHealthPercent`))
        (if (`self.LowHealthEventReady?`)
          (message `/Game/HealthComponents/BP_GeneralInterface.LowHealthEvent` (`self.GetOwner`) (`self.CurrentHealth`) (`self.MaxHealth`))
          (if (> (`self.LowHealthPercentEventCoolDown`) 0.0)
            (if (not (`KismetSystemLibrary.K2_IsValidTimerHandle` (`self.LowHealthEventCoolDownHandle`)))
              (bind _returnvalue (`KismetSystemLibrary.K2_SetTimer` self "ResetLowHealthEventReadyVirible" (`self.LowHealthPercentEventCoolDown`)))
              (set `self.LowHealthEventCoolDownHandle` _returnvalue)
              ;[1 1 1] 大于等于0进入冷却，否则无冷却
              (set `self.LowHealthEventReady?` false)
              (if (`self.bUseDebug`)
                (`KismetSystemLibrary.PrintString` "低生命值事件触发并开始冷却"))))
          (elif (`self.bUseDebug`)
            (`KismetSystemLibrary.PrintString` "低生命值事件冷却未完成" true true (struct :`R` 1.0 :`G` 0.016463 :`A` 1.0) 0.01)
            (return)
            (else
              (return))))
        (else
          (return)))
      (else
        (return)))))

(fn `CreateHealthBar`
  (`/Engine/EditorBlueprintResources/StandardMacros.IsValid` (`self.HealthBar_UI`)
    (:`Is Not Valid`
      (bind _returnvalue (`|CreateWidget` "/Game/HealthComponents/W_HealthBar.W_HealthBar_C" null self))
      (bind _output_get (set `self.HealthBar_UI` _returnvalue))
      (`UserWidget.AddToViewport` _output_get 0))))

(fn `DeathCalculate`
  (if (<= (`self.CurrentHealth`) 0.0)
    (if (not (`self.bDeath`))
      (set `self.bDeath` true)
      (message `/Game/HealthComponents/BP_GeneralInterface.DeathEvent` (`self.GetOwner`)))))

(fn `IfAutoCreateUI`
  (if (`self.bAutoCreateUIHealthBar`)
    (`self.CreateHealthBar`)))

(fn `OnGotCure`
  (params (HealthValue :type "Float (double-precision)"))
  (`self.BasicCureCalculate` HealthValue)
  (if (`self.bUseCureEvent`)
    (if (`self.bCureEventReady`)
      (message `/Game/HealthComponents/BP_GeneralInterface.OnCureEvent` (`self.GetOwner`) (`self.CurrentHealth`) (`self.MaxHealth`))
      (if (> (`self.CureEventCalculate`) 0.0)
        (set `self.bCureEventReady` false)
        (bind _returnvalue (`KismetSystemLibrary.K2_SetTimer` self "ResetCureEventCoolDown" (`self.CureEventCalculate`)))
        (set `self.CureEventCoolDownHandle` _returnvalue)
        (if (`self.bUseDebug`)
          (`KismetSystemLibrary.PrintString` "治疗事件冷却开始"))))))

(fn `OnGotDamage`
  (params (DamageValue :type "Float (double-precision)"))
  (`self.BasicDamageCaculate` DamageValue)
  (`self.DeathCalculate`))

(fn `ResetCureEventCoolDown`
  (set `self.bCureEventReady` true)
  (`KismetSystemLibrary.K2_ClearAndInvalidateTimerHandle` (`self.CureEventCoolDownHandle`))
  (if (`self.bUseDebug`)
    (`KismetSystemLibrary.PrintString` "治疗事件冷却完成" true true (struct :`R` 1.0 :`G` 0.016463 :`A` 1.0))))

(fn `ResetLowHealthEventReadyVirible`
  (set `self.LowHealthEventReady?` true)
  (`KismetSystemLibrary.K2_ClearAndInvalidateTimerHandle` (`self.LowHealthEventCoolDownHandle`))
  (if (`self.bUseDebug`)
    (`KismetSystemLibrary.PrintString` "低生命值事件冷却完成" true true (struct :`R` 1.0 :`G` 0.016463 :`A` 1.0))))
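; AC_BagCompo is a component that manages the on-screen bag (inventory) UI.
; On BeginPlay it creates a WBP_Bag widget, stores it and adds it to the viewport.
; Pressing Tab flips an open flag and calls the widget's AnimtedConDes with the new state to animate it open or closed.
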(event `self.ReceiveBeginPlay`
  (bind _returnvalue (`|CreateWidget` "/Game/AI_Npc/ShotgunAI_01/Summons/WBP_Bag.WBP_Bag_C"))
  (bind _output_get (set `self.BagUI` _returnvalue))
  (`UserWidget.AddToViewport` _output_get 0))

(event `Key|Tab`
  (params (Key :type "Key Structure"))
  (:`Pressed`
    (if (`self.BngOpen`)
      (`/Game/AI_Npc/ShotgunAI_01/Summons/WBP_Bag.AnimtedCon_Des` (`self.BagUI`) false)
      (set `self.BngOpen` false)
      (else
        (`/Game/AI_Npc/ShotgunAI_01/Summons/WBP_Bag.AnimtedCon_Des` (`self.BagUI`) true)
        (set `self.BngOpen` true)))))
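; BP_Pick is a pickup actor that lets the player add its item to their bag.
; Overlapping its Box shows a widget prompt and enables input, and leaving hides the prompt and disables input.
; Pressing F gets the pawn's bag component through a message call, appends ItemInfo, refreshes the bag UI and destroys the actor.
; BeginPlay creates the WBP_InteractWidget prompt, and a helper function can change its text.
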(event `self.Box.OnComponentBeginOverlap`
  (params (OverlappedComponent :type "PrimitiveComponent Object Reference") (OtherActor :type "Actor Object Reference") (OtherComp :type "PrimitiveComponent Object Reference") (OtherBodyIndex :type Integer) (bFromSweep :type Boolean) (SweepResult :type "HitResult Structure (by ref)"))
  (`SceneComponent.SetHiddenInGame` (`self.Widget`) false false)
  (`self.EnableInput` (`GameplayStatics.GetPlayerController` 0)))

(event `self.Box.OnComponentEndOverlap`
  (params (OverlappedComponent :type "PrimitiveComponent Object Reference") (OtherActor :type "Actor Object Reference") (OtherComp :type "PrimitiveComponent Object Reference") (OtherBodyIndex :type Integer))
  (`SceneComponent.SetHiddenInGame` (`self.Widget`) true false)
  (`self.DisableInput` (`GameplayStatics.GetPlayerController` 0)))

(event `Key|F`
  (params (Key :type "Key Structure"))
  (:`Pressed`
    (bind _bagcompo (message `/Game/AI_Npc/ShotgunAI_01/Summons/BPI_ProjectInterfaces.GetBagComponent` (`GameplayStatics.GetPlayerPawn` 0)))
    (`/Engine/EditorBlueprintResources/StandardMacros.IsValid` _bagcompo
      (:`Is Valid`
        (`KismetArrayLibrary.Array_Add` (`/Game/AI_Npc/ShotgunAI_01/Summons/AC_BagCompo.ST_Bag` _bagcompo) (`self.ItemInfo`))
        (`/Game/AI_Npc/ShotgunAI_01/Summons/WBP_Bag.刷新背包` (`/Game/AI_Npc/ShotgunAI_01/Summons/AC_BagCompo.BagUI` _bagcompo))
        (`self.K2_DestroyActor`)))))

(event `self.ReceiveBeginPlay`
  (bind _returnvalue (`|CreateWidget` "/Game/AI_Npc/ShotgunAI_01/Summons/WBP_InteractWidget.WBP_InteractWidget_C" null "拾取"))
  (`WidgetComponent.SetWidget` (`self.Widget`) _returnvalue))

(fn `UserConstructionScript`)

(fn `修改文字`
  (params (InText :type Text))
  (bind _aswbp_interact_widget (cast `/Game/AI_Npc/ShotgunAI_01/Summons/WBP_InteractWidget` (`WidgetComponent.GetWidget` (`self.Widget`))))
  (`TextBlock.SetText` (`/Game/AI_Npc/ShotgunAI_01/Summons/WBP_InteractWidget.TextBlock_Main` _aswbp_interact_widget) InText))
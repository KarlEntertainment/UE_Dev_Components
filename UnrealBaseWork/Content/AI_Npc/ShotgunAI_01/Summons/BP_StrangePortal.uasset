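; BP_StrangePortal is a temporary, numbered portal that teleports the player to a linked portal.
; On BeginPlay it finds the portal whose number matches its destination number and caches that portal's landing point.
; Any hit on HiddenDoor moves player pawn 0 there.
; Timelines grow the Niagara spawn rate and scale on appearance, then shrink them after a delay before destroying the actor.
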(event `self.ReceiveBeginPlay`
  (bind _niagara (`self.Niagara`))
  (`self.GetTarget`)
  (bind (_direction `_新建轨道_0`) (`Timeline|时间轴` :!via `PlayFromStart`)
    (:`Update`
      (`NiagaraComponent.SetVariableFloat` _niagara "SpawnRate" (`KismetMathLibrary.Lerp` 0.0 7000.0 `_新建轨道_0`))
      (`SceneComponent.SetRelativeScale3D` _niagara (`KismetMathLibrary.VLerp` (0.0 0.0 0.0) (1.0 1.0 1.0) `_新建轨道_0`)))
    (:`Finished`
      (`KismetSystemLibrary.Delay` 10.0)
      (`self.DestroyPortal`))))

(event `DestroyPortal`
  (bind _niagara (`self.Niagara`))
  (bind (_direction `_新建轨道_0`) (`Timeline|时间轴_0` :!via `ReverseFromEnd`)
    (:`Update`
      (`NiagaraComponent.SetVariableFloat` _niagara "SpawnRate" (`KismetMathLibrary.Lerp` 0.0 7000.0 `_新建轨道_0`))
      (`SceneComponent.SetRelativeScale3D` _niagara (`KismetMathLibrary.VLerp` (0.0 0.0 0.0) (1.0 1.0 1.0) `_新建轨道_0`)))
    (:`Finished`
      (`self.K2_DestroyActor`))))

(event `GetTarget`
  (bind _outactors (`GameplayStatics.GetAllActorsOfClass` "BP_StrangePortal_C"))
  (for _array_element _outactors
    (if (== (`/Game/AI_Npc/ShotgunAI_01/Summons/BP_StrangePortal.当前门编号` _array_element) (`self.传送到编号`))
      (bind _output_get (set `self.目标门` _array_element))
      (set `self.目标落点` (`/Game/AI_Npc/ShotgunAI_01/Summons/BP_StrangePortal.玩家落点` _output_get))
      (break))))

(event `self.HiddenDoor.OnComponentHit`
  (params (HitComponent :type "PrimitiveComponent Object Reference") (OtherActor :type "Actor Object Reference") (OtherComp :type "PrimitiveComponent Object Reference") (NormalImpulse :type "Vector Structure") (Hit :type "HitResult Structure (by ref)"))
  (bind `_目标落点` (`self.目标落点`))
  (`self.K2_SetActorLocationAndRotation` (`GameplayStatics.GetPlayerPawn` 0) (`SceneComponent.K2_GetComponentLocation` `_目标落点`) (`SceneComponent.K2_GetComponentRotation` `_目标落点`) false false))

(fn `UserConstructionScript`)
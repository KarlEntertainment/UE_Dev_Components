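; BP_AI_MoveAound is an AI-controlled pawn that runs the BP_AroundAI behavior tree through its AI controller on BeginPlay.
; SetGetBack writes the GetBack blackboard bool when the blackboard is valid, and also clears the Target key when set to true.
; Movement and decision logic are left to the behavior tree, with the pawn only starting it and exposing this blackboard switch.
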(event `self.ReceiveBeginPlay`
  (bind `_asai控制器` (cast `AIController` (`self.GetController`)))
  (`AIController.RunBehaviorTree` `_asai控制器` "/Game/UnrealFrame/BP_AroundAI.BP_AroundAI"))

(fn `SetGetBack`
  (params (BoolValue :type Boolean))
  (bind _returnvalue (`AIBlueprintHelperLibrary.GetBlackboard` null))
  (`/Engine/EditorBlueprintResources/StandardMacros.IsValid` _returnvalue
    (:`Is Valid`
      (`BlackboardComponent.SetValueAsBool` _returnvalue "GetBack" BoolValue)
      (if BoolValue
        (`BlackboardComponent.SetValueAsObject` (`AIBlueprintHelperLibrary.GetBlackboard` null) "Target" null)))))

(fn `UserConstructionScript`)
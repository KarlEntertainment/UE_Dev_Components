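; BP_Pick is a pickup item actor that adds its item to the player's bag when interacted with.
; Its InteractEvent gets the bag component from the player pawn and, if valid, appends ItemInfo to STBag, refreshes the bag UI and destroys the actor.
; The construction script applies the configurable NewMesh to the Cube mesh component, setting each pickup's appearance.
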(event `self.InteractEvent`
  (bind _bagcompo (message `/Game/UnrealFrame/BPI_ProjectInterfaces.GetBagComponent` (`GameplayStatics.GetPlayerPawn` 0)))
  (`/Engine/EditorBlueprintResources/StandardMacros.IsValid` _bagcompo
    (:`Is Valid`
      (`KismetArrayLibrary.Array_Add` (`/Game/UnrealFrame/AC_BagCompo.ST_Bag` _bagcompo) (`self.ItemInfo`))
      (`/Game/UnrealFrame/WBP_Bag.刷新背包` (`/Game/UnrealFrame/AC_BagCompo.BagUI` _bagcompo))
      (`self.K2_DestroyActor`))))

(fn `UserConstructionScript`
  (`StaticMeshComponent.SetStaticMesh` (`self.Cube`) (`self.New Mesh`)))
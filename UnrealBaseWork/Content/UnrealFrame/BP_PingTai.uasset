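; BP_PingTai is an interactable platform (PingTai) that toggles between its starting position and a point 500 units above it.
; BeginPlay calls the parent, then caches the actor's location and the raised target.
; Each InteractEvent flips the InDown flag and uses MoveComponentTo to slide the root component to the matching position over half a second.
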(event `self.ReceiveBeginPlay`
  (bind _returnvalue (`self.K2_GetActorLocation`))
  (`parent.ReceiveBeginPlay`)
  (set `self.InitLocation` _returnvalue)
  (set `self.TargetLocation` (+ _returnvalue (0.0 0.0 500.0))))

(event `self.InteractEvent`
  (if (`self.InDown`)
    (set `self.InDown` false)
    (`KismetSystemLibrary.MoveComponentTo` (`self.RootComponent`) (`self.TargetLocation`) (struct) false false 0.5)
    (else
      (set `self.InDown` true)
      (`KismetSystemLibrary.MoveComponentTo` (`self.RootComponent`) (`self.InitLocation`) (struct) false false 0.5))))

(fn `UserConstructionScript`)
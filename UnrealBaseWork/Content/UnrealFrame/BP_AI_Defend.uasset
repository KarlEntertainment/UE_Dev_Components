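; BP_AI_Defend is an AI character that guards a BP_DefendArea found in the level on BeginPlay, where it also starts BT_DefendAI.
; AI perception writes any perceived BP_ThirdPersonCharacter to the blackboard's Target key.
; Tick checks distance to the area and, at or beyond a fixed leash radius, calls SetGetBack to raise the GetBack flag and clear Target.
; Nothing in this Blueprint lowers GetBack.
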(event `self.ReceiveBeginPlay`
  (bind _returnvalue (`GameplayStatics.GetActorOfClass` "/Game/UnrealFrame/BP_DefendArea.BP_DefendArea_C"))
  (set `self.DefendArea` _returnvalue)
  (bind `_asai控制器` (cast `AIController` (`self.GetController`)))
  (`AIController.RunBehaviorTree` `_asai控制器` "/Game/UnrealFrame/BT_DefendAI.BT_DefendAI"))

(event `self.ReceiveTick`
  (params (DeltaSeconds :type "Float (single-precision)"))
  (if (>= (`self.GetDistanceTo` self (`self.DefendArea`)) 500.0)
    (`self.SetGetBack` true)))

(event `self.AIPerception.OnTargetPerceptionUpdated`
  (params (Actor :type "Actor Object Reference") (Stimulus :type "AIStimulus Structure"))
  (bind _asbp_third_person_character (cast `/Game/ThirdPerson/Blueprints/BP_ThirdPersonCharacter` Actor))
  (`BlackboardComponent.SetValueAsObject` (`AIBlueprintHelperLibrary.GetBlackboard` null) "Target" _asbp_third_person_character))

(fn `SetGetBack`
  (params (BoolValue :type Boolean))
  (bind _returnvalue (`AIBlueprintHelperLibrary.GetBlackboard` null))
  (`/Engine/EditorBlueprintResources/StandardMacros.IsValid` _returnvalue
    (:`Is Valid`
      (`BlackboardComponent.SetValueAsBool` _returnvalue "GetBack" BoolValue)
      (if BoolValue
        (`BlackboardComponent.SetValueAsObject` (`AIBlueprintHelperLibrary.GetBlackboard` null) "Target" null)))))

(fn `UserConstructionScript`)
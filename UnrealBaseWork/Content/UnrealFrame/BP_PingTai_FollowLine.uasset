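; Platform actor that steps along the points of a linked spline each time it receives an interact event.
; On BeginPlay it finds the BP_SuperSpline whose 编号 matches its 对标编号 and stores it as the target.
; Each InteractEvent advances the reached-point index, or resets it to -1 past the point count, and uses MoveComponentTo to glide the root toward a spline point's world location over a fixed duration.
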(event `self.ReceiveBeginPlay`
  (`parent.ReceiveBeginPlay`)
  (bind _outactors (`GameplayStatics.GetAllActorsOfClass` "/Game/UnrealFrame/BP_SuperSpline.BP_SuperSpline_C"))
  (for _array_element _outactors
    (if (== (`/Game/UnrealFrame/BP_SuperSpline.编号` _array_element) (`self.对标编号`))
      (set `self.目标spline` _array_element)
      (break))))

(event `self.InteractEvent`
  (bind _spline (`/Game/UnrealFrame/BP_SuperSpline.Spline` (`self.目标spline`)))
  (if (>= (`self.当前已抵达Index`) (`SplineComponent.GetNumberOfSplinePoints` _spline))
    (set `self.当前已抵达Index` -1)
    (else
      (bind _result (`/Engine/EditorBlueprintResources/StandardMacros.IncrementInt` (`self.当前已抵达Index`))
        (:`  `
          _))))
  (`KismetSystemLibrary.MoveComponentTo` (`self.RootComponent`) (`SplineComponent.GetLocationAtSplinePoint` _spline _result "World") (struct) false false 0.5))

(fn `UserConstructionScript`)
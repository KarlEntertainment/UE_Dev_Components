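; Figurine viewer actor for the virtual exhibition hall that shows a selected item's mesh for mouse-drag inspection.
; 修改网格创建UI copies the target's mesh and opens the WBP_ShouBan info widget, whose event triggers ShowEvent to swap in WBP_ZhanShi and enable input.
; A SceneCapture2D renders only that mesh, which left-drag rotates in yaw and pitch.
; 移除展示UI后续事件 closes the viewer, resets rotation, returns input to the pawn and restores the info widget.
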(event `Key|LeftMouseButton`
  (params (Key :type "Key Structure"))
  (:`Pressed`
    (set `self.鼠标按下` true))
  (:`Released`
    (set `self.鼠标按下` false)))

(event `InputAxisKey|MouseX`
  (params (AxisValue :type "Float (single-precision)"))
  (if (`self.鼠标按下`)
    (`SceneComponent.K2_AddRelativeRotation` (`self.StaticMesh`) (`KismetMathLibrary.MakeRotator` 0.0 0.0 AxisValue) false false)))

(event `InputAxisKey|MouseY`
  (params (AxisValue :type "Float (single-precision)"))
  (if (`self.鼠标按下`)
    (`SceneComponent.K2_AddRelativeRotation` (`self.StaticMesh`) (`KismetMathLibrary.MakeRotator` 0.0 AxisValue) false false)))

(event `ShowEvent`
  (`Widget.RemoveFromParent` (`self.ShouBanUI`))
  (set `self.ShouBanUI` null)
  (`self.EnableInput` (`GameplayStatics.GetPlayerController` 0))
  (bind _returnvalue (`|CreateWidget` "/Game/虚拟展馆/Mesh/第六展厅/手办/WBP_ZhanShi.WBP_ZhanShi_C" null self))
  (bind _output_get (set `self.ZhanShiUI` _returnvalue))
  (`UserWidget.AddToViewport` _output_get 0))

(fn `UserConstructionScript`
  (`SceneCaptureComponent.ShowOnlyComponent` (`self.SceneCaptureComponent2D`) (`self.StaticMesh`))
  (`SceneComponent.K2_SetRelativeLocation` (`self.SpringArm`) (`self.RelativeLocation`) false false))

(fn `修改网格创建UI`
  (params (`目标` :type "StaticMeshComponent Object Reference") (ST_ItemInfo :type "/Game/UnrealFrame/ST_ItemInfo Structure (by ref)"))
  (bind _output_get (set `self.当前物品信息` ST_ItemInfo))
  (`/Engine/EditorBlueprintResources/StandardMacros.IsValid` (`self.ZhanShiUI`)
    (:`Is Not Valid`
      (`StaticMeshComponent.SetStaticMesh` (`self.StaticMesh`) (`StaticMeshComponent.StaticMesh` `目标`))
      (bind (`_物品名字` `_物品图片` `_物品信息`) (break `/Game/UnrealFrame/ST_ItemInfo` _output_get))
      (bind _returnvalue (`|CreateWidget` "/Game/虚拟展馆/Mesh/第六展厅/手办/WBP_ShouBan.WBP_ShouBan_C" null `_物品名字` `_物品信息`))
      (bind _output_get_2 (set `self.ShouBanUI` _returnvalue))
      (`UserWidget.AddToViewport` _output_get_2 0)
      (add `/Game/虚拟展馆/Mesh/第六展厅/手办/WBP_ShouBan.CallShowEvent` _output_get_2 (`|CreateDelegate` :!event `ShowEvent`)))))

(fn `移除展示UI后续事件`
  (bind (`_物品名字` `_物品图片` `_物品信息`) (break `/Game/UnrealFrame/ST_ItemInfo` (`self.当前物品信息`)))
  (`Widget.RemoveFromParent` (`self.ZhanShiUI`))
  (set `self.ZhanShiUI` null)
  (`self.EnableInput` (`GameplayStatics.GetPlayerPawn` 0) (`GameplayStatics.GetPlayerController` 0))
  (`SceneComponent.K2_SetRelativeRotation` :`self` (`self.StaticMesh`))
  (`self.DisableInput` (`GameplayStatics.GetPlayerController` 0))
  (bind _returnvalue (`|CreateWidget` "/Game/虚拟展馆/Mesh/第六展厅/手办/WBP_ShouBan.WBP_ShouBan_C" null `_物品名字` `_物品信息`))
  (bind _output_get (set `self.ShouBanUI` _returnvalue))
  (`UserWidget.AddToViewport` _output_get 0)
  (add `/Game/虚拟展馆/Mesh/第六展厅/手办/WBP_ShouBan.CallShowEvent` _output_get (`|CreateDelegate` :!event `ShowEvent`)))